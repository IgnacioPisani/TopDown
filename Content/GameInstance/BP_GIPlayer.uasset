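; Game instance that manages slot-based saves and keeps the active save across level changes.
; On Init it loads or creates an SG_Data object for each slot name, tracking existing saves in a separate array.
; LoadGame opens RoomLevel and sets the current save plus a flag that lets NeedLoadGame return its struct.
; CleanSaveGame resets a slot with the current date and writes it to disk through SaveGame.
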(event `self.ReceiveInit`
  (bind _savegamearray (`self.SaveGameArray`))
  (for _array_element (`self.SlotName`)
    (bind _returnvalue (`GameplayStatics.DoesSaveGameExist` _array_element))
    (if _returnvalue
      (bind _returnvalue_2 (`GameplayStatics.LoadGameFromSlot` _array_element))
      (bind _assg_data (cast `/Game/Save/SG_Data` _returnvalue_2))
      (bind _output_get (set `self.SaveG` _assg_data))
      (`KismetArrayLibrary.Array_AddUnique` (`self.SaveGameArray`) _output_get)
      (`KismetArrayLibrary.Array_AddUnique` (`self.ExistingSaveGameArray`) _output_get)
      (else
        (bind _returnvalue_3 (`GameplayStatics.CreateSaveGameObject` "/Game/Save/SG_Data.SG_Data_C"))
        (bind _output_get_2 (set `self.SaveG` _returnvalue_3))
        (bind _returnvalue_4 (`KismetArrayLibrary.Array_AddUnique` _savegamearray _output_get_2))
        (`/Game/Save/SG_Data.SetStruct` (`|GetArrayItem` _savegamearray _returnvalue_4) (make `/Game/Structure/S_Save` "-870.000000,1888.000000,100.000000|0.000000,0.000000,0.000000|1.000000,1.000000,1.000000"))))))

(fn `CleanSaveGame`
  (params (CleanSave :type Integer))
  (locals (NewLocalVar :type "/Game/Save/SG_Data Object Reference"))
  (bind _output (`|GetArrayItem` (`self.SaveGameArray`) CleanSave))
  (`/Game/Save/SG_Data.SetStruct` _output (make `/Game/Structure/S_Save` "-870.000000,1888.000000,100.000000|0.000000,0.000000,0.000000|1.000000,1.000000,1.000000" 3.0 (`KismetMathLibrary.Now`) true))
  (bind _output_get (set `self.CurrentSave` _output))
  (set `self.CurrentName` (`|GetArrayItem` (`self.SlotName`) CleanSave))
  (bind _newparam (`/Game/Save/SG_Data.GetStruct` _output_get))
  (`self.SaveGame` _newparam)
  (`KismetArrayLibrary.Array_AddUnique` (`self.ExistingSaveGameArray`) _output_get))

(fn `GameToSave`
  (params (Slot :type Integer) (SavesGame :type "Array of /Game/Save/SG_Data Object Reference"))
  (returns (`IsSaveLoaded?` :type Boolean))
  (bind _newparam (`/Game/Save/SG_Data.GetStruct` (`|GetArrayItem` SavesGame Slot)))
  (return (`.bIsLoaded?_16_1FAF69B741CB615C908E048206E249F1` (break `/Game/Structure/S_Save` _newparam))))

(fn `Get Game Saves`
  (returns (NewParam :type "Array of /Game/Save/SG_Data Object Reference"))
  (return (`self.SaveGameArray`)))

(fn `GetExistingSaves`
  (returns (ExistingSaveGameArray :type "Array of /Game/Save/SG_Data Object Reference"))
  (return (`self.ExistingSaveGameArray`)))

(fn `LoadGame`
  (params (Slot :type Integer) (SavesGame :type "Array of /Game/Save/SG_Data Object Reference"))
  (`GameplayStatics.OpenLevel` "RoomLevel")
  (set `self.CurrentSave` (`|GetArrayItem` SavesGame Slot))
  (set `self.CurrentName` (`|GetArrayItem` (`self.SlotName`) Slot))
  (set `self.bSaveLoad?` true))

(fn `NeedLoadGame`
  (returns (S_Save :type "/Game/Structure/S_Save Structure"))
  (if (`self.bSaveLoad?`)
    (bind _newparam (`/Game/Save/SG_Data.GetStruct` (`self.CurrentSave`)))
    (return _newparam)))

(fn `SaveGame`
  (params (Struct :type "/Game/Structure/S_Save Structure"))
  (bind _currentsave (`self.CurrentSave`))
  (`/Game/Save/SG_Data.SetStruct` _currentsave Struct)
  (bind _returnvalue (`GameplayStatics.SaveGameToSlot` _currentsave (`self.CurrentName`)))
  (if _returnvalue
    _))