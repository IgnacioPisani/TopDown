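; BP_SwitchTarget is a shootable switch that triggers a linked bridge.
; When a BP_Projectile overlaps Box2, a dot product of the projectile-to-target direction and the actor's forward vector limits valid hits to projectiles behind the target, relative to its forward.
; A valid hit calls ShowBridgeMessage on BridgeToActivate and destroys the target.
; The dot value is printed for every projectile overlap.
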(event `self.Box2.OnComponentBeginOverlap`
  (params (OverlappedComponent :type "PrimitiveComponent Object Reference") (OtherActor :type "Actor Object Reference") (OtherComp :type "PrimitiveComponent Object Reference") (OtherBodyIndex :type Integer) (bFromSweep :type Boolean) (SweepResult :type "HitResult Structure (by ref)"))
  (bind _asbp_projectile (cast `/Game/Blueprints/Projectile/BP_Projectile` OtherActor))
  (bind _returnvalue (`KismetMathLibrary.Dot_VectorVector` (`KismetMathLibrary.Normal` (- (`self.K2_GetActorLocation`) (`self.K2_GetActorLocation` _asbp_projectile))) (`self.GetActorForwardVector`)))
  (`KismetSystemLibrary.PrintString` (`KismetStringLibrary.Conv_DoubleToString` _returnvalue))
  (if (> _returnvalue 0.4)
    (message `/Game/Blueprints/Bridge/Interfaces/BPI_ShowBridge.ShowBridge` (`self.BridgeToActivate`))
    (`self.K2_DestroyActor`)))

(fn `UserConstructionScript`)