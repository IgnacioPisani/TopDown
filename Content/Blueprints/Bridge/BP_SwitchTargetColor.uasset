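; BP_SwitchTargetColor is a shootable switch target that picks a blue, red or black sprite at BeginPlay from its color enum.
; When a BP_Projectile overlaps its box, a dot product against the forward vector accepts only hits from behind that vector.
; A valid hit passes the switch name to the player character's SaveBridgesMessage, calls ShowBridgeMessage on the linked bridge, then destroys the target.
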(event `self.ReceiveBeginPlay`
  (switch `/Game/Blueprints/Bridge/E_Color` (`self.E_Color`)
    (:`NewEnumerator0`
      (`PaperSpriteComponent.SetSprite` (`self.PaperSprite`) "/Game/TILESET/TilesFINAL4_Sprite_15.TilesFINAL4_Sprite_15"))
    (:`NewEnumerator1`
      (`PaperSpriteComponent.SetSprite` (`self.PaperSprite`) "/Game/TILESET/TilesFINAL4_Sprite_16.TilesFINAL4_Sprite_16"))
    (:`NewEnumerator2`
      (`PaperSpriteComponent.SetSprite` (`self.PaperSprite`) "/Game/TILESET/TilesFINAL4_Sprite_14.TilesFINAL4_Sprite_14"))))

(event `self.Box2.OnComponentBeginOverlap`
  (params (OverlappedComponent :type "PrimitiveComponent Object Reference") (OtherActor :type "Actor Object Reference") (OtherComp :type "PrimitiveComponent Object Reference") (OtherBodyIndex :type Integer) (bFromSweep :type Boolean) (SweepResult :type "HitResult Structure (by ref)"))
  (bind _asbp_projectile (cast `/Game/Blueprints/Projectile/BP_Projectile` OtherActor))
  (if (> (`KismetMathLibrary.Dot_VectorVector` (`KismetMathLibrary.Normal` (- (`self.K2_GetActorLocation`) (`self.K2_GetActorLocation` _asbp_projectile))) (`self.GetActorForwardVector`)) 0.0)
    (message `/Game/Blueprints/Characters/Character/Interfaces/BPI_SaveBridges.Save Bridges` (`GameplayStatics.GetPlayerCharacter` 0) (`self.SwitchTargetName`))
    (message `/Game/Blueprints/Bridge/Interfaces/BPI_ShowBridge.ShowBridge` (`self.BridgeToActivate`))
    (`self.K2_DestroyActor`)))

(fn `UserConstructionScript`)