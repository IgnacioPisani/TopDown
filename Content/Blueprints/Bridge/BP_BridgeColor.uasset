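; BP_BridgeColor is a color-coded bridge actor that can rise into view.
; On BeginPlay, its EColor value picks the blue, red or black tile sprite for the PaperSprite component.
; The ShowBridge event plays the BridgeRise timeline, which keeps X and Y from the world location and sets relative Z directly to the ZOffset curve value, not adding it to the starting height.
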(event `self.ReceiveBeginPlay`
  (switch `/Game/Blueprints/Bridge/E_Color` (`self.E_Color`)
    (:`NewEnumerator0`
      (`PaperSpriteComponent.SetSprite` (`self.PaperSprite`) "/Game/TILESET/TilesFINAL3_Sprite_2.TilesFINAL3_Sprite_2"))
    (:`NewEnumerator1`
      (`PaperSpriteComponent.SetSprite` (`self.PaperSprite`) "/Game/TILESET/TilesFINAL3_Sprite_1.TilesFINAL3_Sprite_1"))
    (:`NewEnumerator2`
      (`PaperSpriteComponent.SetSprite` (`self.PaperSprite`) "/Game/TILESET/TilesFINAL3_Sprite_0.TilesFINAL3_Sprite_0"))))

(event `self.ShowBridge`
  (bind (_returnvalue_x _returnvalue_y) (`KismetMathLibrary.BreakVector` (`self.K2_GetActorLocation`)))
  (bind (_direction _zoffset) (`Timeline|BridgeRise`)
    (:`Update`
      (`self.K2_SetActorRelativeLocation` (`KismetMathLibrary.MakeVector` _returnvalue_x _returnvalue_y _zoffset)))))

(fn `UserConstructionScript`)