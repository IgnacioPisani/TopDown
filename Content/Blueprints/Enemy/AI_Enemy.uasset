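; AI_Enemy is the AI controller for enemy pawns, starting the BT_Enemy behavior tree on BeginPlay.
; When Pawn Sensing sees a pawn, it writes a seen BP_Character into a blackboard key as the target object.
; If the controlled BP_Enemy is dead at that moment, it clears that key instead.
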(event `self.ReceiveBeginPlay`
  (`self.RunBehaviorTree` "/Game/Blueprints/Enemy/BT_Enemy.BT_Enemy"))

(event `self.ReceiveTick`
  (params (DeltaSeconds :type "Float (single-precision)")))

(event `self.PawnSensing.OnSeePawn`
  (params (Pawn :type "Pawn Object Reference"))
  (bind _key_name (`self.Key Name`))
  (bind _asbp_enemy (cast `/Game/Blueprints/Enemy/BP_Enemy` (`self.K2_GetPawn`)))
  (if (`/Game/Blueprints/Enemy/BP_Enemy.IsDeath?` _asbp_enemy)
    (`BlackboardComponent.ClearValue` (`AIBlueprintHelperLibrary.GetBlackboard` null) _key_name)
    (else
      (bind _asbp_character (cast `/Game/Blueprints/Character/BP_Character` Pawn))
      (`BlackboardComponent.SetValueAsObject` (`AIBlueprintHelperLibrary.GetBlackboard` null) _key_name _asbp_character))))

(fn `UserConstructionScript`)