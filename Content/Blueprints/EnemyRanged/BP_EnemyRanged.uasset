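; Ranged enemy that tracks a player character entering its detection sphere and can fire projectiles at it.
; Sphere overlap stores the target and sets a shooting flag; leaving clears the flag and the "Shoot" timer.
; SpawnProjectile offsets the muzzle toward the target and snaps projectile rotation to four cardinal directions by dominant axis.
; Nothing here starts that timer, calls SpawnProjectile or sets the ProjectileDirection used for velocity.
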(event `self.Sphere.OnComponentBeginOverlap`
  (params (OverlappedComponent :type "PrimitiveComponent Object Reference") (OtherActor :type "Actor Object Reference") (OtherComp :type "PrimitiveComponent Object Reference") (OtherBodyIndex :type Integer) (bFromSweep :type Boolean) (SweepResult :type "HitResult Structure (by ref)"))
  (bind _asbp_character (cast `/Game/Blueprints/Character/BP_Character` OtherActor))
  (set `self.BP CharacterReference` _asbp_character)
  (`self.StartAttacking`))

(event `StartAttacking`
  (if (not (`self.IsShooting?`))
    (set `self.IsShooting?` true)))

(event `self.Sphere.OnComponentEndOverlap`
  (params (OverlappedComponent :type "PrimitiveComponent Object Reference") (OtherActor :type "Actor Object Reference") (OtherComp :type "PrimitiveComponent Object Reference") (OtherBodyIndex :type Integer))
  (cast `/Game/Blueprints/Character/BP_Character` OtherActor)
  (set `self.IsShooting?` false)
  (`KismetSystemLibrary.K2_ClearTimer` null "Shoot"))

(fn `SetProjectileRotation`
  (bind (_directionality_x _directionality_y) (`KismetMathLibrary.BreakVector2D` (`self.Directionality`)))
  (bind (_returnvalue_x _returnvalue_y) (`KismetMathLibrary.BreakVector` (`KismetMathLibrary.MakeVector` _directionality_x (* _directionality_y -1.0))))
  (if (> (`KismetMathLibrary.Abs` _returnvalue_x) (`KismetMathLibrary.Abs` _returnvalue_y))
    (if (> _returnvalue_x 0.0)
      (set `self.ProjectileRotation` (struct))
      (else
        (set `self.ProjectileRotation` (struct :`Yaw` 180.0))))
    (elif (> _returnvalue_y 0.0)
      (set `self.ProjectileRotation` (struct :`Yaw` 90.0))
      (else
        (set `self.ProjectileRotation` (struct :`Yaw` -90.0))))))

(fn `SpawnProjectile`
  (bind (_returnvalue_location _returnvalue_rotation _returnvalue_scale) (`KismetMathLibrary.BreakTransform` (`self.GetTransform`)))
  (bind (_directionality_x _directionality_y) (`KismetMathLibrary.BreakVector2D` (`self.Directionality`)))
  (bind (_returnvalue_x _returnvalue_y) (`KismetMathLibrary.BreakVector` (`KismetMathLibrary.Normal` (- (`self.K2_GetActorLocation` (`self.BP CharacterReference`)) (`self.K2_GetActorLocation`)))))
  (set `self.Directionality` (`KismetMathLibrary.MakeVector2D` _returnvalue_x (* _returnvalue_y -1.0)))
  (`self.SetProjectileRotation`)
  (`|SpawnActorFromClass` "/Game/Blueprints/ProjectileEnemy/BP_ProjectileEnemy.BP_ProjectileEnemy_C" (`KismetMathLibrary.MakeTransform` (+ (* (`KismetMathLibrary.MakeVector` _directionality_x (* _directionality_y -1.0)) (`self.MuzzleOffset`)) _returnvalue_location) (`self.ProjectileRotation`) _returnvalue_scale) "Undefined" "MultiplyWithRoot" null (* (`self.ProjectileDirection`) (`self.ProjectileSpeed`)) null))

(fn `UserConstructionScript`)