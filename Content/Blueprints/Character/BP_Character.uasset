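; Player character for a top-down, sprite-based game with move, melee hit, roll and shoot actions via Enhanced Input.
; Move input stores a direction that aims the roll's launch and the spawned projectile.
; Boolean flags with timed resets keep hit, roll and shoot mutually exclusive.
; HandleHit damages enemies in a debug-drawn box sized by sprite sockets, but this graph never runs it; IA_Hit only sets its flag.
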(event `self.ReceiveBeginPlay`
  (bind _asplayer_controller (cast `PlayerController` (`self.GetController`)))
  (message `EnhancedInputSubsystemInterface.AddMappingContext` (pcsubsystem `EnhancedInputLocalPlayerSubsystem` _asplayer_controller) "/Game/Input/IMC_TopDown.IMC_TopDown" 0 (struct)))

(event `EnhancedInput|/Game/Input/Actions/IA_Move`
  (params (ActionValue :type "Vector2D Structure") (ElapsedSeconds :type "Float (double-precision)") (TriggeredSeconds :type "Float (double-precision)") (InputAction :type "InputAction Object Reference" :default "/Game/Input/Actions/IA_Move.IA_Move"))
  (bind (_x _y) (`KismetMathLibrary.BreakVector2D` ActionValue))
  (:`Triggered`
    (`self.AddMovementInput` (1.0 0.0 0.0) _x)
    (`self.AddMovementInput` (0.0 -1.0 0.0) _y)
    (set `self.Directionality` (`KismetMathLibrary.MakeVector2D` _x _y))))

(event `EnhancedInput|/Game/Input/Actions/IA_Hit`
  (params (ActionValue :type Boolean) (ElapsedSeconds :type "Float (double-precision)") (TriggeredSeconds :type "Float (double-precision)") (InputAction :type "InputAction Object Reference" :default "/Game/Input/Actions/IA_Hit.IA_Hit"))
  (:`Triggered`
    (if (not (or (`self.IsShooting?`) (`self.IsRolling?`) (`self.IsHitting?`)))
      (set `self.IsHitting?` true)
      (`KismetSystemLibrary.Delay` 0.25)
      (set `self.IsHitting?` false))))

(event `EnhancedInput|/Game/Input/Actions/IA_Roll`
  (params (ActionValue :type Boolean) (ElapsedSeconds :type "Float (double-precision)") (TriggeredSeconds :type "Float (double-precision)") (InputAction :type "InputAction Object Reference" :default "/Game/Input/Actions/IA_Roll.IA_Roll"))
  (bind (_directionality_x _directionality_y) (`KismetMathLibrary.BreakVector2D` (`self.Directionality`)))
  (:`Triggered`
    (if (not (or (`self.IsShooting?`) (`self.IsRolling?`) (`self.IsHitting?`)))
      (set `self.IsRolling?` true)
      (`self.LaunchCharacter` (* (`KismetMathLibrary.MakeVector` _directionality_x (* _directionality_y -1.0)) (`self.RollSpeed`)) true)
      (`KismetSystemLibrary.Delay` 0.5)
      (set `self.IsRolling?` false))))

(event `EnhancedInput|/Game/Input/Actions/IA_Shoot`
  (params (ActionValue :type Boolean) (ElapsedSeconds :type "Float (double-precision)") (TriggeredSeconds :type "Float (double-precision)") (InputAction :type "InputAction Object Reference" :default "/Game/Input/Actions/IA_Shoot.IA_Shoot"))
  (bind (_returnvalue_location _returnvalue_rotation _returnvalue_scale) (`KismetMathLibrary.BreakTransform` (`self.GetTransform`)))
  (bind (_directionality_x _directionality_y) (`KismetMathLibrary.BreakVector2D` (`self.Directionality`)))
  (bind (_directionality_x_2 _directionality_y_2) (`KismetMathLibrary.BreakVector2D` (`self.Directionality`)))
  (:`Started`
    (if (not (or (`self.IsShooting?`) (`self.IsRolling?`) (`self.IsHitting?`)))
      (set `self.IsShooting?` true)
      (`|SpawnActorFromClass` "/Game/Blueprints/Projectile/BP_Projectile.BP_Projectile_C" (`KismetMathLibrary.MakeTransform` (+ (* (`KismetMathLibrary.MakeVector` _directionality_x_2 (* _directionality_y_2 -1.0)) (`self.MuzzleOffset`)) _returnvalue_location) _returnvalue_rotation _returnvalue_scale) "Undefined" "MultiplyWithRoot" null (* (`KismetMathLibrary.Normal` (`KismetMathLibrary.MakeVector` _directionality_x (* _directionality_y -1.0))) (`self.ProjectileSpeed`)) null)
      (`KismetSystemLibrary.Delay` 0.5)
      (set `self.IsShooting?` false))))

(fn `HandleHit`
  (bind _returnvalue_location (`KismetMathLibrary.BreakTransform` (`SceneComponent.GetSocketTransform` (`self.Sprite`) "HitSocketSize" "RTS_ParentBoneSpace")))
  (bind _returnvalue (`SceneComponent.GetSocketLocation` (`self.Sprite`) "HitSocket"))
  (`KismetSystemLibrary.DrawDebugBox` _returnvalue _returnvalue_location (struct :`R` 1.0 :`G` 0.691271 :`B` 0.2456 :`A` 1.0) (struct) 0.0 5.0)
  (bind _outactors (`KismetSystemLibrary.BoxOverlapActors` _returnvalue _returnvalue_location (`|MakeArray` "ObjectTypeQuery3" :!type "EObjectTypeQuery Enum") "/Game/Blueprints/Enemy/BP_Enemy.BP_Enemy_C"))
  (for _array_element _outactors
    (`GameplayStatics.ApplyDamage` _array_element (`self.Damage`))))

(fn `UserConstructionScript`)