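; BP_Key is a collectible colored key built with Paper2D.
; On BeginPlay, its color enum selects a blue or purple sprite.
; When its sphere overlaps an actor implementing BPI_GetKey, it passes its key name through that interface and destroys itself, so it needs no cast to the collector's class.
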(event `self.ReceiveBeginPlay`
  (switch `/Game/Blueprints/Items/E_ColorKey` (`self.E_ColorKey`)
    (:`NewEnumerator0`
      (`PaperSpriteComponent.SetSprite` (`self.PaperSprite`) "/Game/TILESET/TilesFINAL5_Sprite_11.TilesFINAL5_Sprite_11"))
    (:`NewEnumerator1`
      (`PaperSpriteComponent.SetSprite` (`self.PaperSprite`) "/Game/TILESET/TilesFINAL5_Sprite_22.TilesFINAL5_Sprite_22"))))

(event `self.Sphere.OnComponentBeginOverlap`
  (params (OverlappedComponent :type "PrimitiveComponent Object Reference") (OtherActor :type "Actor Object Reference") (OtherComp :type "PrimitiveComponent Object Reference") (OtherBodyIndex :type Integer) (bFromSweep :type Boolean) (SweepResult :type "HitResult Structure (by ref)"))
  (if (`KismetSystemLibrary.DoesImplementInterface` OtherActor "/Game/Blueprints/Characters/Character/Interfaces/BPI_GetKey.BPI_GetKey_C")
    (message `/Game/Blueprints/Characters/Character/Interfaces/BPI_GetKey.GetKey` OtherActor (`self.KeyName`))
    (`self.K2_DestroyActor`)))

(fn `UserConstructionScript`)