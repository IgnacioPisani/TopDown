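; BP_Dreamcatcher is an item that ends the current level when a qualifying actor touches its Sphere trigger.
; The overlap accepts any actor implementing BPI_GetKey, using the interface only as a filter without calling it.
; It shows the BPW_NextChapter widget and switches to UI-only input.
; After a short delay it restores game input, opens MainMenu_Level and destroys itself.
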(event `self.ReceiveBeginPlay`)

(event `self.Sphere.OnComponentBeginOverlap`
  (params (OverlappedComponent :type "PrimitiveComponent Object Reference") (OtherActor :type "Actor Object Reference") (OtherComp :type "PrimitiveComponent Object Reference") (OtherBodyIndex :type Integer) (bFromSweep :type Boolean) (SweepResult :type "HitResult Structure (by ref)"))
  (if (`KismetSystemLibrary.DoesImplementInterface` OtherActor "/Game/Blueprints/Characters/Character/Interfaces/BPI_GetKey.BPI_GetKey_C")
    (bind _returnvalue (`|CreateWidget` "/Game/UI/Menus/Final/BPW_NextChapter.BPW_NextChapter_C"))
    (`UserWidget.AddToViewport` _returnvalue 0)
    (`WidgetBlueprintLibrary.SetInputMode_UIOnlyEx` (`GameplayStatics.GetPlayerController` 0) null)
    (`KismetSystemLibrary.Delay` 3.0)
    (`WidgetBlueprintLibrary.SetInputMode_GameOnly` (`GameplayStatics.GetPlayerController` 0))
    (`GameplayStatics.OpenLevel` "MainMenu_Level")
    (`self.K2_DestroyActor`)))

(fn `UserConstructionScript`)