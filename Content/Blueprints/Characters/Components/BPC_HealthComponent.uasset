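; BPC_HealthComponent is a character component that tracks health and death state.
; DecreaseHealth and IncreaseHealth adjust Health, clamp it between MinHealth and MaxHealth, and broadcast OnLifeChanged with the current and max values.
; DecreaseHealth also sets IsDeath and fires OnDeath once when health drops to zero or below, while IncreaseHealth never clears that flag.
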(fn `DecreaseHealth`
  (params (Damage :type "Float (double-precision)"))
  (bind _maxhealth (`self.MaxHealth`))
  (bind _output_get (set `self.Health` (`KismetMathLibrary.FClamp` (- (`self.Health`) Damage) (`self.MinHealth`) _maxhealth)))
  (`self.OnLifeChanged` _output_get _maxhealth)
  (if (and (<= _output_get 0.0) (not (`self.bIsDeath?`)))
    (set `self.bIsDeath?` true)
    (`self.OnDeath`)))

(fn `IncreaseHealth`
  (params (HealthPoints :type "Float (double-precision)"))
  (bind _maxhealth (`self.MaxHealth`))
  (bind _output_get (set `self.Health` (`KismetMathLibrary.FClamp` (+ HealthPoints (`self.Health`)) (`self.MinHealth`) _maxhealth)))
  (`self.OnLifeChanged` _output_get _maxhealth))