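; Player character for a 2D-sprite action game with four-way facing, melee, roll, shooting, healing, coins, key and respawn point.
; PaperZD animation overrides set state flags that gate actions, while HandleHit damages enemies and HandleSpawnShoot fires projectiles along the facing direction.
; Damage triggers knockback with timed stun and blinking invulnerability; death reloads the level.
; BeginPlay grants weapon and key, signals overlapping camera boxes, and restores saved health, facing and position from the GameInstance.
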(event `self.ReceiveBeginPlay`
  ;[1 1 1] Event BeginPlay
  (`parent.ReceiveBeginPlay`)
  (set `self.bHasWeapon?` true)
  (set `self.bHasKey?` true)
  (bind _outactors (`GameplayStatics.GetAllActorsOfClass` "/Game/Blueprints/CameraBox/BP_CameraBox.BP_CameraBox_C"))
  (for _array_element _outactors
    (if (`self.IsOverlappingActor` _array_element)
      (`self.CameraChanged` _array_element)))
  (bind _asbp_giplayer (cast `/Game/GameInstance/BP_GIPlayer` (`GameplayStatics.GetGameInstance`)))
  (bind _output_get (set `self.As BP GIPlayer` _asbp_giplayer))
  (bind _s_save (`/Game/GameInstance/BP_GIPlayer.NeedLoadGame` _output_get))
  (`self.LoadGameForCharacter` _s_save))

(event `/Game/Blueprints/Characters/Character/Interfaces/BPI_Move.Move`
  (params (ActionValue :type "Vector2D Structure"))
  (bind (_x _y) (`KismetMathLibrary.BreakVector2D` ActionValue))
  ;[1 1 1] Move
  (if (not (or (`/Game/Blueprints/Characters/Components/BPC_HealthComponent.bIsDeath?` (`self.BPC_HealthComponent`)) (`self.bIsShooting?`) (`self.bIsAttacking?`) (`self.bIsStunned?`)))
    (`self.AddMovementInput` (1.0 0.0 0.0) _x)
    (`self.AddMovementInput` (0.0 1.0 0.0) _y)
    (if (> (`KismetMathLibrary.Abs` _x) (`KismetMathLibrary.Abs` _y))
      (if (> _x 0.0)
        (set `self.Directionality` (1.0 0.0))
        (else
          (set `self.Directionality` (-1.0 0.0))))
      (elif (> _y 0.0)
        (set `self.Directionality` (0.0 1.0))
        (else
          (set `self.Directionality` (0.0 -1.0)))))))

(event `/Game/Blueprints/Characters/Character/Interfaces/BPI_Attack.Attack`
  ;[1 1 1] Hit
  (if (not (or (`self.bIsShooting?`) (`self.bIsRolling?`) (`self.bIsAttacking?`) (`/Game/Blueprints/Characters/Components/BPC_HealthComponent.bIsDeath?` (`self.BPC_HealthComponent`)) (`self.bIsStunned?`)))
    (`PaperZDPlaySlotOverrideAction.PlayAnimationOverrideWithCallbacks` (`PaperZDAnimationComponent.AnimInstance` (`self.AnimationComponent`)) "/Game/Blueprints/Characters/Character/AnimSequences/Hit.Hit"
      (:`then`
        (set `self.bIsAttacking?` true))
      (:`OnCompleted`
        (set `self.bIsAttacking?` false :!label _label))
      (:`OnCancelled`
        (goto _label)))))

(event `/Game/Blueprints/Characters/Character/Interfaces/BPI_Roll.Roll`
  (bind (_directionality_x _directionality_y) (`KismetMathLibrary.BreakVector2D` (`self.Directionality`)))
  ;[1 1 1] Roll
  (if (not (or (`self.bIsShooting?`) (`self.bIsRolling?`) (`self.bIsAttacking?`) (`/Game/Blueprints/Characters/Components/BPC_HealthComponent.bIsDeath?` (`self.BPC_HealthComponent`)) (`self.bIsStunned?`)))
    (`GameplayStatics.PlaySound2D` "/Game/Sound/SFX/Character/DashPrueba.DashPrueba" 1.0 1.0 0.0 null null)
    (`PaperZDPlaySlotOverrideAction.PlayAnimationOverrideWithCallbacks` (`PaperZDAnimationComponent.AnimInstance` (`self.AnimationComponent`)) "/Game/Blueprints/Characters/Character/AnimSequences/Roll.Roll"
      (:`then`
        (set `self.bIsRolling?` true)
        (`self.LaunchCharacter` (* (`KismetMathLibrary.MakeVector` _directionality_x _directionality_y) (`self.RollSpeed`)) true))
      (:`OnCompleted`
        (set `self.bIsRolling?` false :!label _label_2))
      (:`OnCancelled`
        (goto _label_2)))))

(event `/Game/Blueprints/Characters/Character/Interfaces/BPI_Shoot.Shoot`
  ;[1 1 1] Shoot
  (if (not (or (`self.bIsShooting?`) (`self.bIsRolling?`) (`self.bIsAttacking?`) (`/Game/Blueprints/Characters/Components/BPC_HealthComponent.bIsDeath?` (`self.BPC_HealthComponent`)) (`self.bIsStunned?`) (not (`self.bHasWeapon?`))))
    (`GameplayStatics.PlaySound2D` "/Game/Sound/SFX/Character/Attaque/Laser.Laser" 1.0 1.0 0.0 null null)
    (`PaperZDPlaySlotOverrideAction.PlayAnimationOverrideWithCallbacks` (`PaperZDAnimationComponent.AnimInstance` (`self.AnimationComponent`)) "/Game/Blueprints/Characters/Character/AnimSequences/Shoot.Shoot"
      (:`then`
        (set `self.bIsShooting?` true))
      (:`OnCompleted`
        (set `self.bIsShooting?` false :!label _label_3))
      (:`OnCancelled`
        (goto _label_3)))))

(event `/Game/Blueprints/Characters/Character/Interfaces/BPI_GetRecoveryItem.GetRecoveryItem`
  (params (HealthPoints :type "Float (double-precision)"))
  ;[1 1 1] RecoveryHealth
  (`/Game/Blueprints/Characters/Components/BPC_HealthComponent.IncreaseHealth` (`self.BPC_HealthComponent`) HealthPoints)
  (bind _returnvalue (`NiagaraFunctionLibrary.SpawnSystemAttached` (`self.System Template`) (`self.Sprite`) "None" (0.0 0.0 0.0) (struct) "KeepRelativeOffset"))
  (`KismetSystemLibrary.Delay` 3.0)
  (`ActorComponent.Deactivate` _returnvalue))

(event `self.OnDeath`
  ;[1 1 1] Death
  (`MovementComponent.StopMovementImmediately` (`self.CharacterMovement`))
  (`PaperZDPlaySlotOverrideAction.PlayAnimationOverrideWithCallbacks` (`PaperZDAnimationComponent.AnimInstance` (`self.AnimationComponent`)) "/Game/Blueprints/Characters/Character/AnimSequences/Death.Death"
    (:`OnCompleted`
      (`self.SetActorHiddenInGame` true)
      (bind _returnvalue (`GameplayStatics.GetCurrentLevelName` true))
      (`GameplayStatics.OpenLevel` (`KismetStringLibrary.Conv_StringToName` _returnvalue)))))

(event `/Game/Blueprints/Characters/Character/Interfaces/BPI_GetCoin.Add Coin`
  (set `self.Coins` (+ 1 (`self.Coins`))))

(event `self.OnLifeChanged`
  (params (Health :type "Float (double-precision)") (MaxHealth :type "Float (double-precision)"))
  (`self.OnLifeChangedHud` Health MaxHealth))

(event `self.OnReceiveDamage`
  (params (Damage :type "Float (double-precision)") (DamageCauser :type "Actor Object Reference"))
  (if (not (`self.bIsInvulnerable?`))
    (`parent.OnReceiveDamage` Damage DamageCauser)
    (`self.ApplyKnockback` DamageCauser)))

(event `ApplyKnockback`
  (params (DamageCauser :type "Actor Object Reference"))
  (bind (_returnvalue_x _returnvalue_y) (`KismetMathLibrary.BreakVector` (* (`KismetMathLibrary.Normal` (- (`self.K2_GetActorLocation`) (`self.K2_GetActorLocation` DamageCauser))) (`self.KnockbackSpeed`))))
  (if (not (`/Game/Blueprints/Characters/Components/BPC_HealthComponent.bIsDeath?` (`self.BPC_HealthComponent`)))
    (`self.StartBlinking`)
    (set `self.bIsInvulnerable?` true)
    (set `self.bIsStunned?` true)
    (`self.LaunchCharacter` (`KismetMathLibrary.MakeVector` _returnvalue_x _returnvalue_y) true)
    (`KismetSystemLibrary.K2_SetTimerDelegate` (delegate `EndInvulnerability`) (`self.TimeInvulnerability`))
    (`KismetSystemLibrary.K2_SetTimerDelegate` (delegate `EndStun`) (`self.TimeStun`))))

(event `EndInvulnerability`
  (set `self.bIsInvulnerable?` false)
  (`self.StopBlinking`)
  (`KismetSystemLibrary.K2_ClearTimer` null "EndInvulnerability"))

(event `EndStun`
  (set `self.bIsStunned?` false)
  (`KismetSystemLibrary.K2_ClearTimer` null "EndStun"))

(event `StartBlinking`
  (`KismetSystemLibrary.K2_SetTimerDelegate` (delegate `ToggleVisibility`) 0.1 true))

(event `ToggleVisibility`
  (`/Engine/EditorBlueprintResources/StandardMacros.FlipFlop`
    (:`A`
      (`self.SetActorHiddenInGame` true))
    (:`B`
      (`self.SetActorHiddenInGame` false))))

(event `StopBlinking`
  (`self.SetActorHiddenInGame` false)
  (`KismetSystemLibrary.K2_ClearTimer` null "ToggleVisibility"))

(event `/Game/Blueprints/Characters/Character/Interfaces/BPI_GetGun.GetGun`
  (set `self.bHasWeapon?` true))

(event `/Game/Blueprints/Characters/Character/Interfaces/BPI_GetKey.GetKey`
  (set `self.bHasKey?` true))

(event `/Game/Blueprints/Characters/Character/Interfaces/BPI_SetRespawnPoint.SetRespawnPoint`
  (params (RespawnPoint :type "Vector Structure"))
  (set `self.RespawnPoint` RespawnPoint))

(event `/Game/Blueprints/Characters/Character/Interfaces/BPI_Respawn.Respawn`
  (`self.K2_SetActorLocation` (`self.RespawnPoint`)))

(event `/Game/Blueprints/Characters/Character/Interfaces/BPI_CameraChanged.OverlapCameraChanged`
  (params (Camera :type "Actor Object Reference"))
  (`self.CameraChanged` Camera))

(fn `HandleHit`
  (bind _returnvalue_location (`KismetMathLibrary.BreakTransform` (`SceneComponent.GetSocketTransform` (`self.Sprite`) "HitSocketSize" "RTS_Actor")))
  (`parent.HandleHit`)
  (`KismetSystemLibrary.BoxOverlapActors` (`SceneComponent.GetSocketLocation` (`self.Sprite`) "HitSocket") _returnvalue_location (`|MakeArray` "ObjectTypeQuery3" :!type "EObjectTypeQuery Enum") "/Game/Blueprints/Characters/Enemies/BP_EnemyBase.BP_EnemyBase_C")
  (for _array_element (`PrimitiveComponent.GetOverlappingActors` (`self.HitBox`) "/Game/Blueprints/Characters/Enemies/BP_EnemyBase.BP_EnemyBase_C")
    (`GameplayStatics.ApplyDamage` _array_element (`self.Damage`))))

(fn `HandleSpawnShoot`
  (bind (_returnvalue_location _returnvalue_rotation _returnvalue_scale) (`KismetMathLibrary.BreakTransform` (`self.GetTransform`)))
  (bind (_directionality_x _directionality_y) (`KismetMathLibrary.BreakVector2D` (`self.Directionality`)))
  (`parent.HandleSpawnShoot`)
  (`self.Set Rotator`)
  (`|SpawnActorFromClass` "/Game/Blueprints/Projectile/BP_Projectile.BP_Projectile_C" (`KismetMathLibrary.MakeTransform` (`SceneComponent.GetSocketLocation` (`self.Sprite`) "ShootSocket") (`self.Rotator`) _returnvalue_scale) "Undefined" "MultiplyWithRoot" null (* (`KismetMathLibrary.MakeVector` _directionality_x _directionality_y) (`self.ProjectileSpeed`)) null))

(fn `HasKey `
  (returns (`bHasKey?` :type Boolean))
  (return (`self.bHasKey?`)))

(fn `LoadGameForCharacter`
  (params (S_Save :type "/Game/Structure/S_Save Structure"))
  (bind _output_get (set `self.SaveStructure` S_Save))
  (set `/Game/Blueprints/Characters/Components/BPC_HealthComponent.Health` (`.CurrentHealth_10_00235DA448B78C8D9515E6993340AD44` (break `/Game/Structure/S_Save` _output_get)) (`self.BPC_HealthComponent`))
  (set `self.Directionality` (`.Directionality_19_3376DF63436EDFF53BB780A707C53BA6` (break `/Game/Structure/S_Save` _output_get)))
  (`self.K2_SetActorLocation` (.location (break `/Game/Structure/S_Save` _output_get))))

(fn `Set Rotator`
  (bind (_directionality_x _directionality_y) (`KismetMathLibrary.BreakVector2D` (`self.Directionality`)))
  (bind (_directionality_x_2 _directionality_y_2) (`KismetMathLibrary.BreakVector2D` (`self.Directionality`)))
  (bind _directionality_x_3 (`KismetMathLibrary.BreakVector2D` (`self.Directionality`)))
  (if (> _directionality_x_2 _directionality_y_2)
    (if (== _directionality_x_3 1.0)
      (set `self.Rotator` (struct :`Roll` 180.0))
      (else
        (set `self.Rotator` (struct :`Pitch` 180.0))))
    (elif (== _directionality_y 1.0)
      (set `self.Rotator` (struct :`Pitch` -180.0))
      (else
        (set `self.Rotator` (struct :`Roll` -180.0))))))

(fn `UserConstructionScript`)