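; Player controller for the top-down character that forwards Enhanced Input actions to BP_Character and manages the HUD, pause menu, camera and saving.
; It creates the health HUD and binds to the character's life and camera-change events.
; ChangeMap teleports the character behind a screen fade, while PlayCamera and StopCamera detach the spring arm and lerp it back on a timeline.
; SaveGame packs the character's transform, health and progress into a structure for the game instance.
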(event `self.ReceiveBeginPlay`
  (bind _bp_characterreference (`self.BP_CharacterReference`))
  (bind _bpc_healthcomponent (`/Game/Blueprints/Characters/BP_CharacterBase.BPC_HealthComponent` _bp_characterreference))
  ;[1 1 1] Event BeginPlay
  (message `EnhancedInputSubsystemInterface.AddMappingContext` (pcsubsystem `EnhancedInputLocalPlayerSubsystem` self) "/Game/Input/IMC_TopDown.IMC_TopDown" 0 (struct))
  (bind _asbp_character (cast `/Game/Blueprints/Characters/Character/BP_Character` (`self.K2_GetPawn`)))
  (set `self.BP_CharacterReference` _asbp_character)
  (bind _returnvalue (`|CreateWidget` "/Game/UI/HUD/BPW_Hud.BPW_Hud_C"))
  (set `self.HealtBarVar` _returnvalue)
  (`UserWidget.AddToViewport` _returnvalue 0)
  (`/Game/UI/HUD/BPW_Hud.UpdateHealthBar` (`self.HealtBarVar`) (`/Game/Blueprints/Characters/Components/BPC_HealthComponent.MaxHealth` _bpc_healthcomponent) (`/Game/Blueprints/Characters/Components/BPC_HealthComponent.Health` _bpc_healthcomponent))
  (add `/Game/Blueprints/Characters/Character/BP_Character.OnLifeChangedHud` _bp_characterreference (delegate `ChangeLifeHud`))
  (add `/Game/Blueprints/Characters/Character/BP_Character.CameraChanged` (`self.BP_CharacterReference`) (delegate `ChangeCamera`))
  (bind _asbp_giplayer (cast `/Game/GameInstance/BP_GIPlayer` (`GameplayStatics.GetGameInstance`)))
  (set `self.BP_GameInstanceReference` _asbp_giplayer))

(event `ChangeLifeHud`
  (params (Health :type "Float (double-precision)") (MaxHealth :type "Float (double-precision)"))
  ;[1 1 1] Event BeginPlay
  (`/Game/UI/HUD/BPW_Hud.UpdateHealthBar` (`self.HealtBarVar`) MaxHealth Health))

(event `ChangeCamera`
  (params (Camera :type "Actor Object Reference"))
  ;[1 1 1] Event BeginPlay
  (`self.SetCamera` Camera))

(event `EnhancedInput|/Game/Input/Actions/IA_Hit`
  (params (ActionValue :type Boolean) (ElapsedSeconds :type "Float (double-precision)") (TriggeredSeconds :type "Float (double-precision)") (InputAction :type "InputAction Object Reference" :default "/Game/Input/Actions/IA_Hit.IA_Hit"))
  ;[1 1 1] Hit
  (:`Started`
    (message `/Game/Blueprints/Characters/Character/Interfaces/BPI_Attack.Attack` (`self.BP_CharacterReference`))))

(event `EnhancedInput|/Game/Input/Actions/IA_Roll`
  (params (ActionValue :type Boolean) (ElapsedSeconds :type "Float (double-precision)") (TriggeredSeconds :type "Float (double-precision)") (InputAction :type "InputAction Object Reference" :default "/Game/Input/Actions/IA_Roll.IA_Roll"))
  ;[1 1 1] Roll
  (:`Started`
    (message `/Game/Blueprints/Characters/Character/Interfaces/BPI_Roll.Roll` (`self.BP_CharacterReference`))))

(event `EnhancedInput|/Game/Input/Actions/IA_Shoot`
  (params (ActionValue :type Boolean) (ElapsedSeconds :type "Float (double-precision)") (TriggeredSeconds :type "Float (double-precision)") (InputAction :type "InputAction Object Reference" :default "/Game/Input/Actions/IA_Shoot.IA_Shoot"))
  ;[1 1 1] Shoot
  (:`Started`
    (message `/Game/Blueprints/Characters/Character/Interfaces/BPI_Shoot.Shoot` (`self.BP_CharacterReference`))))

(event `EnhancedInput|/Game/Input/Actions/IA_Move`
  (params (ActionValue :type "Vector2D Structure") (ElapsedSeconds :type "Float (double-precision)") (TriggeredSeconds :type "Float (double-precision)") (InputAction :type "InputAction Object Reference" :default "/Game/Input/Actions/IA_Move.IA_Move"))
  ;[1 1 1] Move
  (:`Triggered`
    (message `/Game/Blueprints/Characters/Character/Interfaces/BPI_Move.Move` (`self.BP_CharacterReference`) ActionValue)))

(event `/Game/Blueprints/Characters/Character/Interfaces/BPI_ChangeMap.ChangeMap`
  (params (MapLocation :type "Vector Structure") (`bHasCharacterCamera?` :type Boolean))
  (bind _bp_characterreference (`self.BP_CharacterReference`))
  (bind _charactermovement (`Character.CharacterMovement` (`self.BP_CharacterReference`)))
  ;[1 1 1] ChangeMap
  (`CharacterMovementComponent.SetMovementMode` _charactermovement "MOVE_None" 0)
  (`MovementComponent.StopMovementImmediately` _charactermovement)
  (`PlayerCameraManager.StartCameraFade` (`self.PlayerCameraManager`) 0.0 1.0 0.5 (struct :`R` 1.0 :`G` 1.0 :`B` 1.0 :`A` 1.0) false true)
  (`Widget.SetVisibility` (`self.HealtBarVar`) "Hidden")
  (`KismetSystemLibrary.Delay` 1.0)
  (`PlayerCameraManager.StartCameraFade` (`self.PlayerCameraManager`) 1.0 0.0 0.5 (struct :`R` 1.0 :`G` 1.0 :`B` 1.0 :`A` 1.0) false true)
  (`Widget.SetVisibility` (`self.HealtBarVar`) "Visible")
  (`self.K2_SetActorLocation` _bp_characterreference MapLocation false true)
  (if `bHasCharacterCamera?`
    (`self.SetCamera` _bp_characterreference)
    (`KismetSystemLibrary.Delay` 0.4))
  (`CharacterMovementComponent.SetMovementMode` _charactermovement "MOVE_Walking" 0))

(event `EnhancedInput|/Game/Input/Actions/IA_PauseGame`
  (params (ActionValue :type Boolean) (ElapsedSeconds :type "Float (double-precision)") (TriggeredSeconds :type "Float (double-precision)") (InputAction :type "InputAction Object Reference" :default "/Game/Input/Actions/IA_PauseGame.IA_PauseGame"))
  (:`Started`
    (if (not (`self.Is Pause Menu Oppened?`))
      (set `self.Is Pause Menu Oppened?` true)
      (bind _returnvalue (`|CreateWidget` "/Game/UI/Menus/PauseMenu/WBP_PauseMenuSwitch.WBP_PauseMenuSwitch_C" self))
      (bind _output_get (set `self.PauseMenuWidget` _returnvalue))
      (`UserWidget.AddToViewport` _output_get 0)
      (`WidgetBlueprintLibrary.SetInputMode_GameAndUIEx` self (`self.PauseMenuWidget`))
      (set `self.bShowMouseCursor` true)
      (`GameplayStatics.SetGamePaused` true)
      (else
        (set `self.Is Pause Menu Oppened?` false)
        (`self.ResumeGame`)))))

(event `/Game/Blueprints/Characters/Character/Interfaces/BPI_ResumeGame.Resume `
  (`self.ResumeGame`))

(event `/Game/Blueprints/Characters/Character/Interfaces/BPI_PlayCamera.PlayCamera`
  (bind _springarm (`/Game/Blueprints/Characters/Character/BP_Character.SpringArm` (`self.BP_CharacterReference`)))
  (set `self.TransformSpringArm` (`SceneComponent.GetRelativeTransform` _springarm))
  (`SceneComponent.K2_DetachFromComponent` _springarm "KeepWorld" "KeepRelative" "KeepRelative" true))

(event `/Game/Blueprints/Characters/Character/Interfaces/BPI_StopCamera.StopCamera`
  (bind _bp_characterreference (`self.BP_CharacterReference`))
  (bind _rootcomponent (`Actor.RootComponent` _bp_characterreference))
  (bind _springarm (`/Game/Blueprints/Characters/Character/BP_Character.SpringArm` _bp_characterreference))
  (bind (_direction _alpha) (`Timeline|TL_Camera` :!via `PlayFromStart`)
    (:`Update`
      (`SceneComponent.K2_SetWorldLocation` _springarm (`KismetMathLibrary.VLerp` (`SceneComponent.K2_GetComponentLocation` _springarm) (`SceneComponent.K2_GetComponentLocation` _rootcomponent) _alpha) false false))
    (:`Finished`
      (`SceneComponent.K2_AttachToComponent` _springarm _rootcomponent "None" "KeepRelative" "KeepWorld" "KeepRelative" true)
      (`SceneComponent.K2_SetRelativeTransform` _springarm (`self.TransformSpringArm`) false false))))

(event `/Game/Blueprints/Characters/Character/Interfaces/BPI_Save.Save`
  (`self.SaveGame`))

(fn `ResumeGame`
  (set `self.Is Pause Menu Oppened?` false)
  (`Widget.RemoveFromParent` (`self.PauseMenuWidget`))
  (`GameplayStatics.SetGamePaused` false)
  (`WidgetBlueprintLibrary.SetInputMode_GameOnly` self)
  (set `self.bShowMouseCursor` false))

(fn `SaveGame`
  (bind _bp_characterreference (`self.BP_CharacterReference`))
  (bind _output_get (set `/Game/Blueprints/Characters/Character/BP_Character.SaveStructure` (make `/Game/Structure/S_Save` (`self.GetTransform` _bp_characterreference) (`/Game/Blueprints/Characters/Components/BPC_HealthComponent.Health` (`/Game/Blueprints/Characters/BP_CharacterBase.BPC_HealthComponent` _bp_characterreference)) (`KismetMathLibrary.Now`) true (`/Game/Blueprints/Characters/BP_CharacterBase.Directionality` _bp_characterreference) (`/Game/Blueprints/Characters/Character/BP_Character.bHasWeapon?` _bp_characterreference) (`/Game/Blueprints/Characters/Character/BP_Character.Coins` _bp_characterreference) (`/Game/Blueprints/Characters/Character/BP_Character.CoinNames` _bp_characterreference) (`/Game/Blueprints/Characters/Character/BP_Character.EnemyNames` _bp_characterreference) (`/Game/Blueprints/Characters/Character/BP_Character.SwitchTargetNames` _bp_characterreference) (`/Game/Blueprints/Characters/Character/BP_Character.RecoveryItemNames` _bp_characterreference) (`/Game/Blueprints/Characters/Character/BP_Character.KeyNames` _bp_characterreference) (`/Game/Blueprints/Characters/Character/BP_Character.DoorNames` _bp_characterreference)) _bp_characterreference))
  (`/Game/GameInstance/BP_GIPlayer.SaveGame` (`self.BP_GameInstanceReference`) _output_get))

(fn `SetCamera`
  (params (CameraLevel :type "Actor Object Reference"))
  (`self.SetViewTargetWithBlend` CameraLevel))

(fn `UserConstructionScript`)