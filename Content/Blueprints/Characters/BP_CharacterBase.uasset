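; BP_CharacterBase is a base character Blueprint that provides shared health and damage plumbing, with empty hooks for combat behavior.
; On BeginPlay it binds death and life-change events from BPCHealthComponent to empty handlers.
; AnyDamage routes through OnReceiveDamage, which decreases the component's health.
; Hit and SpawnShoot events forward to empty HandleHit and HandleSpawnShoot functions, and SetDirectionality stores the character's directionality.
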(event `self.ReceiveBeginPlay`
  (bind _bpc_healthcomponent (`self.BPC_HealthComponent`))
  (add `/Game/Blueprints/Characters/Components/BPC_HealthComponent.OnDeath` _bpc_healthcomponent (delegate `OnDeath`))
  (add `/Game/Blueprints/Characters/Components/BPC_HealthComponent.OnLifeChanged` _bpc_healthcomponent (delegate `OnLifeChanged`)))

(event `OnLifeChanged`
  (params (Health :type "Float (double-precision)") (MaxHealth :type "Float (double-precision)")))

(event `OnDeath`)

(event `self.ReceiveAnyDamage`
  (params (Damage :type "Float (single-precision)") (DamageType :type "DamageType Object Reference") (InstigatedBy :type "Controller Object Reference") (DamageCauser :type "Actor Object Reference"))
  (`self.OnReceiveDamage` Damage DamageCauser))

(event `OnReceiveDamage`
  (params (Damage :type "Float (double-precision)") (DamageCauser :type "Actor Object Reference"))
  (`/Game/Blueprints/Characters/Components/BPC_HealthComponent.DecreaseHealth` (`self.BPC_HealthComponent`) Damage))

(event `/Game/Blueprints/Characters/Character/Interfaces/BPI_Hit.Hit`
  (`self.HandleHit`))

(event `/Game/Blueprints/Characters/Character/Interfaces/BPI_SpawnShoot.SpawnShoot`
  (`self.HandleSpawnShoot`))

(fn `HandleHit`)

(fn `HandleSpawnShoot`)

(fn `SetDirectionality`
  (params (Directionality :type "Vector2D Structure"))
  (set `self.Directionality` Directionality))

(fn `UserConstructionScript`)