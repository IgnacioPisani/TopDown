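; Ranged enemy Blueprint with a sprite body that attacks a target location by firing projectiles.
; AttackRange stores the target and plays an Attack animation override, using IsAttacking and the health component's death flag to block re-entry.
; HandleSpawnShoot, extending the parent's version, turns toward the target, updates sprite directionality and spawns BP_ProjectileEnemy at ShootSocket.
; OnDeath disables capsule collision and movement, plays Death, then destroys the actor after a short delay.
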(event `self.OnDeath`
  (bind _charactermovement (`self.CharacterMovement`))
  (`parent.OnDeath`)
  (`PrimitiveComponent.SetCollisionEnabled` (`self.CapsuleComponent`) "NoCollision")
  (`CharacterMovementComponent.SetMovementMode` _charactermovement "MOVE_None" 0)
  (`MovementComponent.StopMovementImmediately` _charactermovement)
  (`PaperZDPlaySlotOverrideAction.PlayAnimationOverrideWithCallbacks` (`PaperZDAnimationComponent.AnimInstance` (`self.AnimationComponent`)) "/Game/Blueprints/Characters/Enemies/EnemyRanged/AnimSequences/Death.Death"
    (:`OnCompleted`
      _)
    (:`OnCancelled`
      _))
  (`KismetSystemLibrary.Delay` 0.2)
  (`self.K2_DestroyActor`))

(event `/Game/Blueprints/Characters/Character/Interfaces/BPI_AttackRange.AttackRange`
  (params (Target :type "Vector Structure"))
  (set `self.TargetLocation` Target)
  (if (and (not (`self.bIsAttacking?`)) (not (`/Game/Blueprints/Characters/Components/BPC_HealthComponent.bIsDeath?` (`self.BPC_HealthComponent`))))
    (`PaperZDPlaySlotOverrideAction.PlayAnimationOverrideWithCallbacks` (`PaperZDAnimationComponent.AnimInstance` (`self.AnimationComponent`)) "/Game/Blueprints/Characters/Enemies/EnemyRanged/AnimSequences/Attack.Attack"
      (:`then`
        (set `self.bIsAttacking?` true))
      (:`OnCompleted`
        (set `self.bIsAttacking?` false :!label _label))
      (:`OnCancelled`
        (goto _label)))))

(fn `HandleSpawnShoot`
  (bind (_returnvalue_location _returnvalue_rotation _returnvalue_scale) (`KismetMathLibrary.BreakTransform` (`self.GetTransform`)))
  (bind _returnvalue (`self.K2_GetActorLocation`))
  (bind _targetlocation (`self.TargetLocation`))
  (bind (_returnvalue_x _returnvalue_y _returnvalue_z) (`KismetMathLibrary.BreakVector` (`KismetMathLibrary.Normal` (- _targetlocation _returnvalue))))
  (`parent.HandleSpawnShoot`)
  (`self.K2_SetActorRotation` (`KismetMathLibrary.FindLookAtRotation` _returnvalue _targetlocation))
  (`self.SetDirectionality` (`KismetMathLibrary.MakeVector2D` _returnvalue_x (* _returnvalue_y -1.0)))
  (`|SpawnActorFromClass` "/Game/Blueprints/ProjectileEnemy/BP_ProjectileEnemy.BP_ProjectileEnemy_C" (`KismetMathLibrary.MakeTransform` (`SceneComponent.GetSocketLocation` (`self.Sprite`) "ShootSocket") (struct) _returnvalue_scale) "Undefined" "MultiplyWithRoot" null (* (`KismetMathLibrary.MakeVector` _returnvalue_x _returnvalue_y _returnvalue_z) (`self.ProjectileSpeed`)) null))

(fn `UserConstructionScript`)