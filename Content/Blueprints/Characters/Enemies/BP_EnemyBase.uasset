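; Base enemy Blueprint that adds a health bar, hit effects and death reporting on top of its parent class.
; BeginPlay caches the BPW_EnemyHealth widget from its widget component, and OnLifeChanged forwards health values to it.
; Taking damage runs the parent logic, then spawns a particle system attached to the Sprite.
; On death, it passes EnemyName to the player character's SaveEnemiesMessage.
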(event `self.ReceiveBeginPlay`
  (`parent.ReceiveBeginPlay`)
  (`self.InitBarHealth`))

(event `self.OnDeath`
  (message `/Game/Blueprints/Characters/Character/Interfaces/BPI_SaveEnemies.SaveEnemies` (`GameplayStatics.GetPlayerCharacter` 0) (`self.EnemyName`)))

(event `self.OnLifeChanged`
  (params (Health :type "Float (double-precision)") (MaxHealth :type "Float (double-precision)"))
  (`self.UpdateHealthBar` Health MaxHealth))

(event `self.ReceiveAnyDamage`
  (params (Damage :type "Float (single-precision)") (DamageType :type "DamageType Object Reference") (InstigatedBy :type "Controller Object Reference") (DamageCauser :type "Actor Object Reference"))
  (`parent.ReceiveAnyDamage` Damage DamageType InstigatedBy DamageCauser)
  (`NiagaraFunctionLibrary.SpawnSystemAttached` (`self.System Template`) (`self.Sprite`) "None" (0.0 0.0 0.0) (struct) "KeepRelativeOffset"))

(fn `InitBarHealth`
  (bind _asbpw_enemy_health (cast `/Game/UI/HUD/BPW_EnemyHealth` (`WidgetComponent.GetUserWidgetObject` (`self.Widget`))))
  (set `self.BPW _EnemyHealthReference` _asbpw_enemy_health))

(fn `UpdateHealthBar`
  (params (Health :type "Float (double-precision)") (MaxHealth :type "Float (double-precision)"))
  (`/Game/UI/HUD/BPW_EnemyHealth.UpdateHealthBar` (`self.BPW _EnemyHealthReference`) Health MaxHealth))

(fn `UserConstructionScript`)