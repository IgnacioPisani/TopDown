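; Boss enemy with three health-based phases, melee and ranged attacks, its own health bar widget, and a Dreamcatcher drop on death.
; Crossing health thirds, and nearly dying, notifies the boss AI controller and boosts walk and projectile speed.
; Animation overrides drive phase-specific shots and invulnerable teleports, with callbacks clearing state flags.
; A burning attack toggles a damage box and lets the capsule pass through pawns.
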(event `self.ReceiveBeginPlay`
  (bind _maxhealth (`/Game/Blueprints/Characters/Components/BPC_HealthComponent.MaxHealth` (`self.BPC_HealthComponent`)))
  (`parent.ReceiveBeginPlay`)
  (set `self.RangeChangePhase` (- _maxhealth (/ _maxhealth 3.0))))

(event `/Game/Blueprints/Characters/Character/Interfaces/BPI_Attack.Attack`
  (if (and (not (`self.bIsAttacking?`)) (not (`/Game/Blueprints/Characters/Components/BPC_HealthComponent.bIsDeath?` (`self.BPC_HealthComponent`))))
    (`PaperZDPlaySlotOverrideAction.PlayAnimationOverrideWithCallbacks` (`PaperZDAnimationComponent.AnimInstance` (`self.AnimationComponent`)) "/Game/Blueprints/Characters/Enemies/EnemyBoss/AnimSequences/Attack.Attack"
      (:`then`
        (set `self.bIsAttacking?` true))
      (:`OnCompleted`
        (set `self.bIsAttacking?` false :!label _label))
      (:`OnCancelled`
        (goto _label)))))

(event `/Game/Blueprints/Characters/Character/Interfaces/BPI_AttackRange.AttackRange`
  (params (Target :type "Vector Structure"))
  (set `self.Target Location` Target)
  (if (and (not (`self.bIsShooting?`)) (not (`/Game/Blueprints/Characters/Components/BPC_HealthComponent.bIsDeath?` (`self.BPC_HealthComponent`))))
    (if (== (`self.CurrentPhase`) 0)
      (`PaperZDPlaySlotOverrideAction.PlayAnimationOverrideWithCallbacks` (`PaperZDAnimationComponent.AnimInstance` (`self.AnimationComponent`)) "/Game/Blueprints/Characters/Enemies/EnemyBoss/AnimSequences/Shoot1.Shoot1"
        (:`then`
          (set `self.bIsShooting?` true :!label _label_2))
        (:`OnCompleted`
          (set `self.bIsShooting?` false :!label _label_3))
        (:`OnCancelled`
          (goto _label_3)))
      (elif (== (`self.CurrentPhase`) 1)
        (`PaperZDPlaySlotOverrideAction.PlayAnimationOverrideWithCallbacks` (`PaperZDAnimationComponent.AnimInstance` (`self.AnimationComponent`)) "/Game/Blueprints/Characters/Enemies/EnemyBoss/AnimSequences/Shoot2.Shoot2"
          (:`then`
            (goto _label_2))
          (:`OnCompleted`
            (goto _label_3))
          (:`OnCancelled`
            (goto _label_3)))
        (else
          (`PaperZDPlaySlotOverrideAction.PlayAnimationOverrideWithCallbacks` (`PaperZDAnimationComponent.AnimInstance` (`self.AnimationComponent`)) "/Game/Blueprints/Characters/Enemies/EnemyBoss/AnimSequences/Shoot3.Shoot3"
            (:`then`
              (goto _label_2))
            (:`OnCompleted`
              (goto _label_3))
            (:`OnCancelled`
              (goto _label_3))))))))

(event `self.OnLifeChanged`
  (params (Health :type "Float (double-precision)") (MaxHealth :type "Float (double-precision)"))
  (`parent.OnLifeChanged` Health MaxHealth)
  (if (and (<= Health (`self.RangeChangePhase`)) (!= (`self.CurrentPhase`) 2))
    (set `self.CurrentPhase` (+ (`self.CurrentPhase`) 1))
    (if (== (`self.CurrentPhase`) 1)
      (set `self.RangeChangePhase` (/ MaxHealth 3.0))
      (`self.ImplementsPhaseBoss` 1.2 (struct :`R` 1.0 :`G` 0.206791 :`A` 1.0) 6.0)
      (else
        (`self.ImplementsPhaseBoss` 2.0 (struct :`R` 1.0 :`A` 1.0) 10.0)))
    (elif (and (< Health 2.0) (not (`self.bIsInTheFinalAttack?`)))
      (`self.ImplementsPhaseBoss` 2.0 (struct :`R` 1.0 :`A` 1.0) 13.0)
      (set `self.bIsInTheFinalAttack?` true))))

(event `self.Box.OnComponentBeginOverlap`
  (params (OverlappedComponent :type "PrimitiveComponent Object Reference") (OtherActor :type "Actor Object Reference") (OtherComp :type "PrimitiveComponent Object Reference") (OtherBodyIndex :type Integer) (bFromSweep :type Boolean) (SweepResult :type "HitResult Structure (by ref)"))
  (if (`KismetSystemLibrary.DoesImplementInterface` OtherActor "/Game/Blueprints/Characters/Character/Interfaces/BPI_Roll.BPI_Roll_C")
    (`GameplayStatics.ApplyDamage` OtherActor (`self.Damage`) null self)))

(event `/Game/Blueprints/Characters/Enemies/EnemyBoss/Interfaces/BPI_FinishAttack.FinishAttack`
  (`self.FinishAttackBoss`))

(event `self.OnReceiveDamage`
  (params (Damage :type "Float (double-precision)") (DamageCauser :type "Actor Object Reference"))
  (if (not (`self.bIsInvulnerable?`))
    (`parent.OnReceiveDamage` Damage DamageCauser)))

(event `/Game/Blueprints/Characters/Enemies/EnemyBoss/Interfaces/BPI_StartAttack.StartAttack`
  (`PrimitiveComponent.SetCollisionResponseToChannel` (`self.CapsuleComponent`) "ECC_Pawn" "ECR_Ignore")
  (`PrimitiveComponent.SetCollisionEnabled` (`self.Box`) "QueryOnly")
  (set `self.bIsBurning?` true))

(event `self.OnDeath`
  (bind _returnvalue (`self.GetTransform`))
  (bind _charactermovement (`self.CharacterMovement`))
  (`parent.OnDeath`)
  (`self.FinishAttackBoss`)
  (`CharacterMovementComponent.SetMovementMode` _charactermovement "MOVE_None" 0)
  (`MovementComponent.StopMovementImmediately` _charactermovement)
  (`PaperZDPlaySlotOverrideAction.PlayAnimationOverrideWithCallbacks` (`PaperZDAnimationComponent.AnimInstance` (`self.AnimationComponent`)) "/Game/Blueprints/Characters/Enemies/EnemyBoss/AnimSequences/Death3.Death3"
    (:`OnCompleted`
      _)
    (:`OnCancelled`
      _))
  (`KismetSystemLibrary.Delay` 0.2)
  (`|SpawnActorFromClass` "/Game/Blueprints/Items/BP_Dreamcatcher.BP_Dreamcatcher_C" (`KismetMathLibrary.MakeTransform` (`KismetMathLibrary.MakeVector` (.x (.location _returnvalue)) (.y (.location _returnvalue)) 20.0) (struct) (.scale _returnvalue)) "Undefined" "MultiplyWithRoot" null null)
  (`self.K2_DestroyActor`))

(event `/Game/Blueprints/Characters/Enemies/EnemyBoss/Interfaces/BPI_Teleport.TeleportBoss`
  (params (Position :type "Vector Structure"))
  (set `self.bIsInvulnerable?` true)
  (if (== (`self.CurrentPhase`) 0)
    (`PaperZDPlaySlotOverrideAction.PlayAnimationOverrideWithCallbacks` (`PaperZDAnimationComponent.AnimInstance` (`self.AnimationComponent`)) "/Game/Blueprints/Characters/Enemies/EnemyBoss/AnimSequences/Death1.Death1"
      (:`OnCompleted`
        _)
      (:`OnCancelled`
        _))
    (elif (== (`self.CurrentPhase`) 1)
      (`PaperZDPlaySlotOverrideAction.PlayAnimationOverrideWithCallbacks` (`PaperZDAnimationComponent.AnimInstance` (`self.AnimationComponent`)) "/Game/Blueprints/Characters/Enemies/EnemyBoss/AnimSequences/Death2.Death2"
        (:`OnCompleted`
          _)
        (:`OnCancelled`
          _))
      (else
        (`PaperZDPlaySlotOverrideAction.PlayAnimationOverrideWithCallbacks` (`PaperZDAnimationComponent.AnimInstance` (`self.AnimationComponent`)) "/Game/Blueprints/Characters/Enemies/EnemyBoss/AnimSequences/Death3.Death3"
          (:`OnCompleted`
            _)
          (:`OnCancelled`
            _)))))
  (`self.K2_SetActorLocation` Position)
  (if (== (`self.CurrentPhase`) 0)
    (`PaperZDPlaySlotOverrideAction.PlayAnimationOverrideWithCallbacks` (`PaperZDAnimationComponent.AnimInstance` (`self.AnimationComponent`)) "/Game/Blueprints/Characters/Enemies/EnemyBoss/AnimSequences/Show1.Show1"
      (:`OnCompleted`
        _)
      (:`OnCancelled`
        _))
    (elif (== (`self.CurrentPhase`) 1)
      (`PaperZDPlaySlotOverrideAction.PlayAnimationOverrideWithCallbacks` (`PaperZDAnimationComponent.AnimInstance` (`self.AnimationComponent`)) "/Game/Blueprints/Characters/Enemies/EnemyBoss/AnimSequences/Show2.Show2"
        (:`OnCompleted`
          _)
        (:`OnCancelled`
          _))
      (else
        (`PaperZDPlaySlotOverrideAction.PlayAnimationOverrideWithCallbacks` (`PaperZDAnimationComponent.AnimInstance` (`self.AnimationComponent`)) "/Game/Blueprints/Characters/Enemies/EnemyBoss/AnimSequences/Show3.Show3"
          (:`OnCompleted`
            _)
          (:`OnCancelled`
            _)))))
  (set `self.bIsInvulnerable?` false))

(fn `FinishAttackBoss`
  (`PrimitiveComponent.SetCollisionEnabled` (`self.Box`) "NoCollision")
  (`PrimitiveComponent.SetCollisionResponseToChannel` (`self.CapsuleComponent`) "ECC_Pawn" "ECR_Block")
  (set `self.bIsBurning?` false))

(fn `HandleHit`
  (`parent.HandleHit`))

(fn `HandleSpawnShoot`
  (bind (_returnvalue_location _returnvalue_rotation _returnvalue_scale) (`KismetMathLibrary.BreakTransform` (`self.GetTransform`)))
  (bind (_returnvalue_x _returnvalue_y _returnvalue_z) (`KismetMathLibrary.BreakVector` (`KismetMathLibrary.Normal` (- (`self.Target Location`) (`self.K2_GetActorLocation`)))))
  (`parent.HandleSpawnShoot`)
  (`|SpawnActorFromClass` "/Game/Blueprints/ProjectileEnemy/BP_ProjectileEnemyBoss.BP_ProjectileEnemyBoss_C" (`KismetMathLibrary.MakeTransform` (`SceneComponent.GetSocketLocation` (`self.Sprite`) "ShootSocket") (struct) _returnvalue_scale) "Undefined" "MultiplyWithRoot" null (* (`KismetMathLibrary.MakeVector` _returnvalue_x _returnvalue_y _returnvalue_z) (* (`self.ProjectileSpeed`) (`self.BoostSpeed`))) null))

(fn `ImplementsPhaseBoss`
  (params (BoastSpeed :type "Float (double-precision)" :default "false") (Color :type "LinearColor Structure" :default "0.0") (TimeTransition :type "Float (double-precision)"))
  (bind _returnvalue (`self.GetController`))
  (bind _charactermovement (`self.CharacterMovement`))
  (if (`KismetSystemLibrary.DoesImplementInterface` _returnvalue "/Game/Blueprints/Characters/Enemies/EnemyBoss/Interfaces/BPI_BossAI.BPI_BossAI_C")
    (message `/Game/Blueprints/Characters/Enemies/EnemyBoss/Interfaces/BPI_BossAI.Enter Phase ` _returnvalue TimeTransition)
    (set `self.BoostSpeed` BoastSpeed)
    (set `CharacterMovementComponent.MaxWalkSpeed` (* (`CharacterMovementComponent.MaxWalkSpeed` _charactermovement) (`self.BoostSpeed`)) _charactermovement)))

(fn `InitBarHealth`
  (bind _returnvalue (`|CreateWidget` "/Game/UI/HUD/BPW_EnemyHealthBoss.BPW_EnemyHealthBoss_C"))
  (bind _output_get (set `self.BPW_EnemyHeathBossReference` _returnvalue))
  (`/Game/UI/HUD/BPW_EnemyHealthBoss.SetName` _output_get (`self.Name`)))

(fn `ShowHealthBar`
  (`UserWidget.AddToViewport` (`self.BPW_EnemyHeathBossReference`) 0))

(fn `UpdateHealthBar`
  (params (Health :type "Float (double-precision)") (MaxHealth :type "Float (double-precision)"))
  (`/Game/UI/HUD/BPW_EnemyHealth.UpdateHealthBar` (`/Game/UI/HUD/BPW_EnemyHealthBoss.BPW_EnemyHealth` (`self.BPW_EnemyHeathBossReference`)) Health MaxHealth))

(fn `UserConstructionScript`
  (`parent.UserConstructionScript`))