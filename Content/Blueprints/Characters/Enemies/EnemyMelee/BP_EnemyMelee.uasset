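; Melee enemy character that attacks with an animation and damages an overlapping player character.
; Attack plays a PaperZD animation override, guarded by an attacking flag and a health component death check.
; HandleHit extends the parent version, applying damage to the first BP_Character overlapping its HitBox.
; OnDeath runs parent logic, halts movement, plays the death animation and destroys the actor after a short delay.
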(event `/Game/Blueprints/Characters/Character/Interfaces/BPI_Attack.Attack`
  (if (and (not (`self.bIsAttacking?`)) (not (`/Game/Blueprints/Characters/Components/BPC_HealthComponent.bIsDeath?` (`self.BPC_HealthComponent`))))
    (`PaperZDPlaySlotOverrideAction.PlayAnimationOverrideWithCallbacks` (`PaperZDAnimationComponent.AnimInstance` (`self.AnimationComponent`)) "/Game/Blueprints/Characters/Enemies/EnemyMelee/AnimSequences/Attack.Attack"
      (:`then`
        (set `self.bIsAttacking?` true))
      (:`OnCompleted`
        (set `self.bIsAttacking?` false :!label _label))
      (:`OnCancelled`
        (goto _label)))))

(event `self.OnDeath`
  (bind _charactermovement (`self.CharacterMovement`))
  (`parent.OnDeath`)
  (`CharacterMovementComponent.SetMovementMode` _charactermovement "MOVE_None" 0)
  (`MovementComponent.StopMovementImmediately` _charactermovement)
  (`PaperZDPlaySlotOverrideAction.PlayAnimationOverrideWithCallbacks` (`PaperZDAnimationComponent.AnimInstance` (`self.AnimationComponent`)) "/Game/Blueprints/Characters/Enemies/EnemyMelee/AnimSequences/Death.Death"
    (:`OnCompleted`
      _)
    (:`OnCancelled`
      _))
  (`KismetSystemLibrary.Delay` 0.2)
  (`self.K2_DestroyActor`))

(fn `HandleHit`
  (`parent.HandleHit`)
  (`GameplayStatics.ApplyDamage` (`|GetArrayItem` (`PrimitiveComponent.GetOverlappingActors` (`self.HitBox`) "/Game/Blueprints/Characters/Character/BP_Character.BP_Character_C")) (`self.Damage`) null self))

(fn `UserConstructionScript`)