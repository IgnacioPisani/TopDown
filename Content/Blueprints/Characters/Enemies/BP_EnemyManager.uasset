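; BP_EnemyManager tracks a list of enemies and drops a gun once all of them have died.
; On BeginPlay it binds a handler to each listed enemy's OnEnemyDied dispatcher.
; Each death removes that enemy from EnemyList, and when the list empties it spawns BP_Gun at the last dead enemy's transform.
; Debug strings print on each death and before the spawn.
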(event `self.ReceiveBeginPlay`
  (for _array_element (`self.EnemyList`)
    (add `/Game/Blueprints/Characters/Enemies/EnemyMelee/BP_EnemyMelee.OnEnemyDied` _array_element (delegate `HandleEnemyDeath`))))

(event `HandleEnemyDeath`
  (params (DeadEnemyReference :type "/Game/Blueprints/Characters/Enemies/EnemyMelee/BP_EnemyMelee Object Reference"))
  (bind _enemylist (`self.EnemyList`))
  (`KismetSystemLibrary.PrintString` "Hello")
  (`KismetArrayLibrary.Array_RemoveItem` _enemylist DeadEnemyReference)
  (if (== (`KismetArrayLibrary.Array_Length` _enemylist) 0)
    (`KismetSystemLibrary.PrintString` "se spawneo?")
    (`|SpawnActorFromClass` "/Game/Blueprints/Items/BP_Gun.BP_Gun_C" (`self.GetTransform` DeadEnemyReference) "Undefined" "MultiplyWithRoot" null null)))

(fn `UserConstructionScript`)