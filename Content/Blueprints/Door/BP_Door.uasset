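; BP_Door is a keyed Paper2D door that moves aside when an actor with the matching key touches it.
; On BeginPlay it picks a blue or black sprite from its color enum and caches its starting location.
; Box1 overlap queries the other actor through BPI_HasKey with key and door names, playing the DoorRise timeline on success.
; The timeline, also triggerable through RiseDoor, offsets the door along Y.
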(event `self.ReceiveBeginPlay`
  (switch `/Game/Blueprints/Bridge/E_Color` (`self.E_Color`)
    (:`NewEnumerator0`
      (`PaperSpriteComponent.SetSprite` (`self.PaperSprite`) "/Game/TILESET/Tiles_Ultimos_Sprite_0.Tiles_Ultimos_Sprite_0"))
    (:`NewEnumerator2`
      (`PaperSpriteComponent.SetSprite` (`self.PaperSprite`) "/Game/TILESET/TilesFINAL4_Sprite_17.TilesFINAL4_Sprite_17")))
  (set `self.DoorLocation` (`self.K2_GetActorLocation`)))

(event `/Game/Blueprints/Door/Interfaces/BPI_RiseDoor.RiseDoor`
  (bind (_doorlocation_x _doorlocation_y) (`KismetMathLibrary.BreakVector` (`self.DoorLocation`)))
  (bind (_direction _newtrack_0) (`Timeline|DoorRise` :!label _label)
    (:`Update`
      (`self.K2_SetActorRelativeLocation` (`KismetMathLibrary.MakeVector` 0.0 (+ _doorlocation_y _newtrack_0))))))

(event `self.Box1.OnComponentBeginOverlap`
  (params (OverlappedComponent :type "PrimitiveComponent Object Reference") (OtherActor :type "Actor Object Reference") (OtherComp :type "PrimitiveComponent Object Reference") (OtherBodyIndex :type Integer) (bFromSweep :type Boolean) (SweepResult :type "HitResult Structure (by ref)"))
  (if (`KismetSystemLibrary.DoesImplementInterface` OtherActor "/Game/Blueprints/Door/Interfaces/BPI_HasKey.BPI_HasKey_C")
    (bind _bhaskey_ (message `/Game/Blueprints/Door/Interfaces/BPI_HasKey.HasKey ` OtherActor (`self.KeyNameReference`) (`self.DoorName`)))
    (if _bhaskey_
      (goto _label))))

(fn `UserConstructionScript`)